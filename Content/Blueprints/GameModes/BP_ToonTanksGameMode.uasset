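; Toon Tanks game mode Blueprint that shows the start and end screens of a match.
; StartGame creates the start game widget and adds it to the viewport.
; GameOver creates the end game widget and uses its WonGame flag to pick victory or death text, with matching text and shadow colors, before displaying it.
; The Blueprint handles only this UI, with BeginPlay, Tick and the construction script left empty.
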(event `self.StartGame`
  (bind _returnvalue (`|CreateWidget` "/Game/Blueprints/Widgets/WBP_StartGameWidget.WBP_StartGameWidget_C"))
  (`UserWidget.AddToViewport` _returnvalue 0))

(event `self.GameOver`
  (params (bWonGame :type Boolean))
  (bind _returnvalue (`|CreateWidget` "/Game/Blueprints/Widgets/WBP_EndGameWidget.WBP_EndGameWidget_C"))
  (bind _displaytext (`/Game/Blueprints/Widgets/WBP_EndGameWidget.DisplayText` _returnvalue))
  (`TextBlock.SetText` _displaytext (select `bool` bWonGame :`false` "You Died!" :`true` "Victory!!" :!type "Text"))
  (`TextBlock.SetColorAndOpacity` _displaytext (select `bool` bWonGame :`false` (`self.FailColor`) :`true` (`self.SuccessColor`)))
  (`TextBlock.SetShadowColorAndOpacity` _displaytext (select `bool` bWonGame :`false` (`self.FailShadowColor`) :`true` (`self.SuccessShadowColor`)))
  (`UserWidget.AddToViewport` _returnvalue 0))

(fn `UserConstructionScript`)